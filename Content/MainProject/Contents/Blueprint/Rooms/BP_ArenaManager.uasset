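; BP_ArenaManager runs a server-authoritative combat arena that locks the exit door until its enemies are dead.
; The combat trigger starts the fight once, counting every BP_ShooterNPC in the level, not just nearby ones, and binding to their health components' death events.
; When the count reaches zero, it unlocks the door and fires OnArenaComplete.
; The exit sensor is bound on BeginPlay to lock the door again.
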(event EventBeginPlay
  (Utilities|FlowControl|Sequence
    (:then_0
      (if (Ability|HasAuthority self)
        (EventDispatchers|BindEventtoOnTriggered (Variables|Default|GetCombatTrigger) (EventDispatchers|CreateEvent self :!event StartCombat))))
    (:then_1
      (if (Ability|HasAuthority self)
        (EventDispatchers|BindEventtoOnTriggered (Variables|Default|GetExitSensor) (EventDispatchers|CreateEvent self :!event LockExitPermanently))))))

(event Collision|EventActorBeginOverlap
  (params (OtherActor :type Actor%20Object%20Reference)))

(event EventTick
  (params (DeltaSeconds :type Float%20%28single-precision%29)))

(fn ConstructionScript)

(fn StartCombat
  (params (TriggeringActor :type Actor%20Object%20Reference))
  (if (Ability|HasAuthority self)
    (if (not (Variables|Default|GetbCombatStarted))
      (Variables|Default|SetbCombatStarted true)
      (Default|Lock (Variables|Default|GetExitDoor))
      (bind _outactors (Actor|GetAllActorsOfClass "/Game/Variant_Shooter/Blueprints/AI/BP_ShooterNPC.BP_ShooterNPC_C"))
      (Variables|Default|SetRemainingEnemyCount (Utilities|Array|Length _outactors))
      (for _array_element _outactors
        (EventDispatchers|BindEventtoOnDeath (Variables|/Game/Variant_Shooter/Blueprints/AI/BP_ShooterNPC.BP_ShooterNPC_C|GetHealthComponent _array_element) (EventDispatchers|CreateEvent self :!event HandleEnemyDeath))))))

(fn HandleEnemyDeath
  (params (Instigator :type Controller%20Object%20Reference) (Causer :type Actor%20Object%20Reference))
  (if (Ability|HasAuthority self)
    (Variables|Default|SetRemainingEnemyCount (- (Variables|Default|GetRemainingEnemyCount) (Class|KismetSystemLibrary|MakeLiteralInteger 1)))
    (if (and (<= (Variables|Default|GetRemainingEnemyCount) (Class|KismetSystemLibrary|MakeLiteralInteger)) (not (Variables|Default|GetbArenaComplete)))
      (Variables|Default|SetbArenaComplete true)
      (Default|Unlock (Variables|Default|GetExitDoor))
      (Default|CallOnArenaComplete))))

(fn LockExitPermanently
  (params (TriggeringActor :type Actor%20Object%20Reference))
  (if (Ability|HasAuthority self)
    (Default|Lock (Variables|Default|GetExitDoor))))