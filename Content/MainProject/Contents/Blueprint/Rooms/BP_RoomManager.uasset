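; Room manager actor that tracks living enemies and signals when the room is cleared.
; On BeginPlay, the authority counts every BP_Enemy_Base in the world, not just in one room, and binds to each one's OnDeath.
; HandleEnemyDeath decrements the remaining count on the authority and calls OnRoomCleared once it reaches zero, with a RoomCleared flag preventing repeat calls.
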(event EventBeginPlay
  (if (Ability|HasAuthority)
    (bind _outactors (Actor|GetAllActorsOfClass "/Game/MainProject/Contents/Blueprint/Enemies/BP_Enemy_Base.BP_Enemy_Base_C"))
    (Variables|Default|SetRemainingEnemyCount (Utilities|Array|Length _outactors))
    (for _array_element _outactors
      (EventDispatchers|BindEventtoOnDeath _array_element (EventDispatchers|CreateEvent :!event HandleEnemyDeath)))))

(event Collision|EventActorBeginOverlap
  (params (OtherActor :type Actor%20Object%20Reference)))

(event EventTick
  (params (DeltaSeconds :type Float%20%28single-precision%29)))

(fn ConstructionScript)

(fn HandleEnemyDeath
  (params (DeadEnemy :type BP%20Enemy%20Base%20Object%20Reference))
  (if (Ability|HasAuthority)
    (Variables|Default|SetRemainingEnemyCount (- (Variables|Default|GetRemainingEnemyCount) (Class|KismetSystemLibrary|MakeLiteralInteger 1)))
    (if (and (<= (Variables|Default|GetRemainingEnemyCount) (Class|KismetSystemLibrary|MakeLiteralInteger)) (not (Variables|Default|GetbRoomCleared)))
      (Variables|Default|SetbRoomCleared true)
      (Default|CallOnRoomCleared))))