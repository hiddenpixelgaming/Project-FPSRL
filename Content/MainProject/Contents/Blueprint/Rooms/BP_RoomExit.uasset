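; BP_RoomExit is a room exit that stays blocked until the room is cleared.
; On BeginPlay it binds to the OnRoomCleared event of the first BP_RoomManager found and turns off collision on its visual mesh.
; When that event fires, Unlock runs only with authority, setting IsUnlocked and disabling the blocking volume's collision.
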(event Custom|HandleRoomCleared
  (CallFunction|Unlock))

(event EventBeginPlay
  (Utilities|FlowControl|Sequence
    (:then_0
      (bind _outactors (Actor|GetAllActorsOfClass "/Game/MainProject/Contents/Blueprint/Rooms/BP_RoomManager.BP_RoomManager_C"))
      (if (> (Utilities|Array|Length _outactors) (Class|KismetSystemLibrary|MakeLiteralInteger))
        (EventDispatchers|BindEventtoOnRoomCleared (Utilities|Array|Get(acopy) _outactors) (EventDispatchers|CreateEvent :!event Custom|HandleRoomCleared))))
    (:then_1
      (Collision|SetCollisionEnabled (Variables|Default|GetVisualMesh) "NoCollision"))))

(event Collision|EventActorBeginOverlap
  (params (OtherActor :type Actor%20Object%20Reference)))

(event EventTick
  (params (DeltaSeconds :type Float%20%28single-precision%29)))

(fn ConstructionScript)

(fn Unlock
  (if (Ability|HasAuthority)
    (Variables|Default|SetbIsUnlocked true)
    (Collision|SetCollisionEnabled (Variables|Default|GetBlockingVolume) "NoCollision")))