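; Multiplayer room door that controls passage through a blocking volume and records which of up to four players have passed.
; Authority-only functions set DoorState, and its OnRep unblocks only when open and not a one-way entrance.
; On overlap, a shooter character's player-state identifier is checked; first-time entrants are marked and their capsule ignores the door while moving.
; End overlap restores blocking, so that bypass works once per player.
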(event EventBeginPlay
  (if (Variables|Default|GetbIsOneWayEntrance)
    (Collision|SetCollisionEnabled (Variables|Default|GetBlockingVolume) "QueryAndPhysics")
    (elif (== (Variables|Default|GetDoorState) (Class|KismetSystemLibrary|MakeLiteralInteger 2))
      (Collision|SetCollisionEnabled (Variables|Default|GetBlockingVolume) "NoCollision")
      (else
        (Collision|SetCollisionEnabled (Variables|Default|GetBlockingVolume) "QueryAndPhysics"))))
  (Collision|SetCollisionEnabled (Variables|Default|GetVisualMesh) "NoCollision"))

(event Collision|EventActorBeginOverlap
  (params (OtherActor :type Actor%20Object%20Reference))
  (CallFunction|HandleDoorOverlap self OtherActor))

(event Collision|EventActorEndOverlap
  (params (OtherActor :type Actor%20Object%20Reference))
  (bind _asbp_shooter_character (Utilities|Casting|CastToBP_ShooterCharacter OtherActor))
  (Collision|IgnoreActorwhenMoving (Variables|/Script/Engine.Character|GetCapsuleComponent _asbp_shooter_character) self false))

(fn ConstructionScript)

(fn OnRepDoorState
  (if (Variables|Default|GetbIsOneWayEntrance)
    (Collision|SetCollisionEnabled (Variables|Default|GetBlockingVolume) "QueryAndPhysics")
    (elif (== (Variables|Default|GetDoorState) (Class|KismetSystemLibrary|MakeLiteralInteger 2))
      (Collision|SetCollisionEnabled (Variables|Default|GetBlockingVolume) "NoCollision")
      (else
        (Collision|SetCollisionEnabled (Variables|Default|GetBlockingVolume) "QueryAndPhysics")))))

(fn Open
  (if (Ability|HasAuthority)
    (if (!= (Variables|Default|GetDoorState) (Class|KismetSystemLibrary|MakeLiteralInteger 4))
      (Variables|Default|SetDoorState 1)
      (Variables|Default|SetDoorState 2))))

(fn Close
  (if (Ability|HasAuthority)
    (if (== (Variables|Default|GetDoorState) (Class|KismetSystemLibrary|MakeLiteralInteger 2))
      (Variables|Default|SetDoorState 3)
      (Variables|Default|SetDoorState 0))))

(fn Lock
  (if (Ability|HasAuthority)
    (Variables|Default|SetDoorState 4)))

(fn Unlock
  (if (Ability|HasAuthority)
    (Variables|Default|SetDoorState 5)
    (Variables|Default|SetDoorState 1)
    (Variables|Default|SetDoorState 2)))

(fn LockOneWay
  (if (Ability|HasAuthority self)
    (Variables|Default|SetDoorState 6)))

(fn HasPlayerPassedDoor
  (params (PlayerIndex :type Integer))
  (if (== PlayerIndex (Class|KismetSystemLibrary|MakeLiteralInteger 1))
    (return (Variables|Default|GetPlayer1Passed))
    (elif (== PlayerIndex (Class|KismetSystemLibrary|MakeLiteralInteger 2))
      (return (Variables|Default|GetPlayer2Passed))
      (elif (== PlayerIndex (Class|KismetSystemLibrary|MakeLiteralInteger 3))
        (return (Variables|Default|GetPlayer3Passed))
        (elif (== PlayerIndex (Class|KismetSystemLibrary|MakeLiteralInteger 4))
          (return (Variables|Default|GetPlayer4Passed))
          (else
            (return false)))))))

(fn MarkPlayerPassedDoor
  (params (PlayerIndex :type Integer))
  (if (Ability|HasAuthority self)
    (if (== PlayerIndex (Class|KismetSystemLibrary|MakeLiteralInteger 1))
      (Variables|Default|SetPlayer1Passed true)
      (elif (== PlayerIndex (Class|KismetSystemLibrary|MakeLiteralInteger 2))
        (Variables|Default|SetPlayer2Passed true)
        (elif (== PlayerIndex (Class|KismetSystemLibrary|MakeLiteralInteger 3))
          (Variables|Default|SetPlayer3Passed true)
          (elif (== PlayerIndex (Class|KismetSystemLibrary|MakeLiteralInteger 4))
            (Variables|Default|SetPlayer4Passed true)))))))

(fn CanPlayerEnterDoor
  (params (PlayerIndex :type Integer))
  (return (not (stale _bhaspassed))))

(fn ValidateDoorEntry
  (params (OtherActor :type Actor%20Object%20Reference))
  (bind _self self)
  (bind (_bisvalid _playerindex) (CallFunction|GetPlayerIdentifierfromActor _self OtherActor))
  (if (not _bisvalid)
    (return false 0)
    (else
      (bind _bcanenter (CallFunction|CanPlayerEnterDoor _self _playerindex))
      (if (not _bcanenter)
        (return false _playerindex)
        (else
          (return true _playerindex))))))

(fn HandleDoorOverlap
  (params (OtherActor :type Actor%20Object%20Reference))
  (bind _self self)
  (bind (_bisvalid _playerindex) (CallFunction|ValidateDoorEntry _self OtherActor))
  (if _bisvalid
    (bind _asbp_shooter_character (Utilities|Casting|CastToBP_ShooterCharacter OtherActor))
    (CallFunction|MarkPlayerPassedDoor _self _playerindex)
    (Collision|IgnoreActorwhenMoving (Variables|/Script/Engine.Character|GetCapsuleComponent _asbp_shooter_character) _self true)))

(fn GetPlayerIdentifierfromActor
  (params (OtherActor :type Actor%20Object%20Reference))
  (bind _asbp_shooter_character (Utilities|Casting|CastToBP_ShooterCharacter OtherActor)
    (:then
      (bind _asbp_player_state_lobby (Utilities|Casting|CastToBP_PlayerStateLobby (Variables|/Script/Engine.Pawn|GetPlayerState _asbp_shooter_character))
        (:then
          (bind _playerindex (Default|GetPlayerIdentifier _asbp_player_state_lobby))
          (return true _playerindex))
        (:CastFailed
          (return false 0))))
    (:CastFailed
      (return false 0))))