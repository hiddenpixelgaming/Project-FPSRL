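; Run manager actor that builds the ordered room sequence for a run from a zone's data.
; GenerateRoomSequence alternates walk and arena picks between fixed spawn, sub-boss, final boss and end-run rooms, then resets the room index.
; Pick helpers draw randomly without replacement, refilling the working pool from the active zone when empty.
; Both helpers are called with a Count of zero, although nine results of each are indexed.
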(event EventBeginPlay)

(event Collision|EventActorBeginOverlap
  (params (OtherActor :type Actor%20Object%20Reference)))

(event EventTick
  (params (DeltaSeconds :type Float%20%28single-precision%29)))

(fn ConstructionScript)

(fn PickRandomWalkRooms
  (params (Count :type Integer))
  (for _index (range 0 (- Count (Class|KismetSystemLibrary|MakeLiteralInteger 1)))
    (if (== (Utilities|Array|Length (LocalVariables|GetWorkingPool)) (Class|KismetSystemLibrary|MakeLiteralInteger))
      (LocalVariables|SetWorkingPool (Variables|/Game/MainProject/Contents/Blueprint/Rooms/BP_ZoneData.BP_ZoneData_C|GetWalkRoomPool (Variables|Default|GetActiveZoneData))))
    (LocalVariables|SetPickIndex (Math|Random|RandomIntegerinRange 0 (- (Utilities|Array|Length (LocalVariables|GetWorkingPool)) (Class|KismetSystemLibrary|MakeLiteralInteger 1))))
    (Utilities|Array|Add (LocalVariables|GetResult) (Utilities|Array|Get(acopy) (LocalVariables|GetWorkingPool) (LocalVariables|GetPickIndex)))
    (Utilities|Array|RemoveIndex (LocalVariables|GetWorkingPool) (LocalVariables|GetPickIndex)))
  (return (LocalVariables|GetResult)))

(fn PickRandomArenaRooms
  (params (Count :type Integer))
  (for _index (range 0 (- Count (Class|KismetSystemLibrary|MakeLiteralInteger 1)))
    (if (== (Utilities|Array|Length (LocalVariables|GetWorkingPool)) (Class|KismetSystemLibrary|MakeLiteralInteger))
      (LocalVariables|SetWorkingPool (Variables|/Game/MainProject/Contents/Blueprint/Rooms/BP_ZoneData.BP_ZoneData_C|GetArenaRoomPool (Variables|Default|GetActiveZoneData))))
    (LocalVariables|SetPickIndex (Math|Random|RandomIntegerinRange 0 (- (Utilities|Array|Length (LocalVariables|GetWorkingPool)) (Class|KismetSystemLibrary|MakeLiteralInteger 1))))
    (Utilities|Array|Add (LocalVariables|GetResult) (Utilities|Array|Get(acopy) (LocalVariables|GetWorkingPool) (LocalVariables|GetPickIndex)))
    (Utilities|Array|RemoveIndex (LocalVariables|GetWorkingPool) (LocalVariables|GetPickIndex)))
  (return (LocalVariables|GetResult)))

(fn GenerateRoomSequence
  (params (Zone :type BP%20Zone%20Data%20Object%20Reference))
  (Variables|Default|SetActiveZoneData Zone)
  (bind _picked (CallFunction|PickRandomWalkRooms))
  (bind _picked_2 (CallFunction|PickRandomArenaRooms))
  (Utilities|Array|Add (Variables|Default|GetRoomSequence) (Variables|/Game/MainProject/Contents/Blueprint/Rooms/BP_ZoneData.BP_ZoneData_C|GetSpawnRoom Zone))
  (Utilities|Array|Add (Variables|Default|GetRoomSequence) (Utilities|Array|Get(acopy) _picked))
  (Utilities|Array|Add (Variables|Default|GetRoomSequence) (Utilities|Array|Get(acopy) _picked_2))
  (Utilities|Array|Add (Variables|Default|GetRoomSequence) (Utilities|Array|Get(acopy) _picked 1))
  (Utilities|Array|Add (Variables|Default|GetRoomSequence) (Utilities|Array|Get(acopy) _picked_2 1))
  (Utilities|Array|Add (Variables|Default|GetRoomSequence) (Utilities|Array|Get(acopy) _picked 2))
  (Utilities|Array|Add (Variables|Default|GetRoomSequence) (Utilities|Array|Get(acopy) _picked_2 2))
  (Utilities|Array|Add (Variables|Default|GetRoomSequence) (Utilities|Array|Get(acopy) _picked 3))
  (Utilities|Array|Add (Variables|Default|GetRoomSequence) (Utilities|Array|Get(acopy) _picked_2 3))
  (Utilities|Array|Add (Variables|Default|GetRoomSequence) (Utilities|Array|Get(acopy) _picked 4))
  (Utilities|Array|Add (Variables|Default|GetRoomSequence) (Utilities|Array|Get(acopy) _picked_2 4))
  (Utilities|Array|Add (Variables|Default|GetRoomSequence) (Variables|/Game/MainProject/Contents/Blueprint/Rooms/BP_ZoneData.BP_ZoneData_C|GetSubBossPrepWalkRoom Zone))
  (Utilities|Array|Add (Variables|Default|GetRoomSequence) (Variables|/Game/MainProject/Contents/Blueprint/Rooms/BP_ZoneData.BP_ZoneData_C|GetSubBossRoom Zone))
  (Utilities|Array|Add (Variables|Default|GetRoomSequence) (Utilities|Array|Get(acopy) _picked 5))
  (Utilities|Array|Add (Variables|Default|GetRoomSequence) (Utilities|Array|Get(acopy) _picked_2 5))
  (Utilities|Array|Add (Variables|Default|GetRoomSequence) (Utilities|Array|Get(acopy) _picked 6))
  (Utilities|Array|Add (Variables|Default|GetRoomSequence) (Utilities|Array|Get(acopy) _picked_2 6))
  (Utilities|Array|Add (Variables|Default|GetRoomSequence) (Utilities|Array|Get(acopy) _picked 7))
  (Utilities|Array|Add (Variables|Default|GetRoomSequence) (Utilities|Array|Get(acopy) _picked_2 7))
  (Utilities|Array|Add (Variables|Default|GetRoomSequence) (Utilities|Array|Get(acopy) _picked 8))
  (Utilities|Array|Add (Variables|Default|GetRoomSequence) (Utilities|Array|Get(acopy) _picked_2 8))
  (Utilities|Array|Add (Variables|Default|GetRoomSequence) (Variables|/Game/MainProject/Contents/Blueprint/Rooms/BP_ZoneData.BP_ZoneData_C|GetFinalBossPrepWalkRoom Zone))
  (Utilities|Array|Add (Variables|Default|GetRoomSequence) (Variables|/Game/MainProject/Contents/Blueprint/Rooms/BP_ZoneData.BP_ZoneData_C|GetFinalBossRoom Zone))
  (Utilities|Array|Add (Variables|Default|GetRoomSequence) (Variables|/Game/MainProject/Contents/Blueprint/Rooms/BP_ZoneData.BP_ZoneData_C|GetEndRunRoom Zone))
  (Variables|Default|SetCurrentRoomIndex 0))