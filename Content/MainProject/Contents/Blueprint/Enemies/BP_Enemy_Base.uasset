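; Base enemy Blueprint that handles taking damage and dying through a health component.
; AnyDamage forwards hits to the HealthComponent, whose health-change event is bound on BeginPlay.
; HandleHealthChanged checks whether the enemy is dead and calls Die, which uses DoOnce to broadcast OnDeath and destroy the actor a single time.
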(event Custom|Die
  (bind _self self)
  (Utilities|FlowControl|DoOnce false
    (:Completed
      (Default|CallOnDeath _self _self)
      (Actor|DestroyActor _self))))

(event EventBeginPlay
  (EventDispatchers|BindEventtoOnHealthChanged (Variables|Default|GetHealthComponent) (EventDispatchers|CreateEvent self :!event HandleHealthChanged)))

(event Collision|EventActorBeginOverlap
  (params (OtherActor :type Actor%20Object%20Reference)))

(event EventTick
  (params (DeltaSeconds :type Float%20%28single-precision%29)))

(event Game|Damage|EventAnyDamage
  (params (Damage :type Float%20%28single-precision%29) (DamageType :type Damage%20Type%20Object%20Reference) (InstigatedBy :type Controller%20Object%20Reference) (DamageCauser :type Actor%20Object%20Reference))
  (Default|HandleTakeAnyDamage (Variables|Default|GetHealthComponent) Damage DamageType InstigatedBy DamageCauser))

(fn ConstructionScript)

(fn HandleHealthChanged
  (params (CurrentHealth :type Float%20%28double-precision%29) (MaxHealth :type Float%20%28double-precision%29))
  (bind _bisdead (Default|IsDead (Variables|Default|GetHealthComponent)))
  (if _bisdead
    (CallFunction|Die self)))