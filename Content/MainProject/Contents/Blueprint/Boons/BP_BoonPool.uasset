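; Boon pool Blueprint that supplies a random selection of boons from its Boons list.
; GetRandomBoons copies the list, then loops until it has Count results or the copy is empty.
; Each pass adds a random item and removes a random index, but Random is evaluated separately for each, so results can repeat.
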(fn GetRandomBoons
  (params (Count :type Integer))
  (LocalVariables|SetWorkingBoons (Variables|Default|GetBoons))
  (while (and (Utilities|Array|IsNotEmpty (LocalVariables|GetWorkingBoons)) (< (Utilities|Array|Length (LocalVariables|GetResult)) Count))
    (Utilities|Array|Add (LocalVariables|GetResult) (.OutItem (Utilities|Array|Random (LocalVariables|GetWorkingBoons))))
    (Utilities|Array|RemoveIndex (LocalVariables|GetWorkingBoons) (.OutIndex (Utilities|Array|Random (LocalVariables|GetWorkingBoons)))))
  (return (LocalVariables|GetResult)))