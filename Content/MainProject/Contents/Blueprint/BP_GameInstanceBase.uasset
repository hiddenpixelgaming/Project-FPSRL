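; Base Game Instance that manages online multiplayer sessions through Advanced Sessions, apparently over Steam.
; It creates a four-slot, game-tagged session and opens the lobby, searches sessions without filtering on that tag, and joins from accepted invites or a pending result.
; Friend invites and joins read pending variables set outside this graph.
; Callbacks update session state, signal search completion and print most failures; leaving ends the session without changing level.
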(event Custom|Create%20Session
  (|AdvancedSession (Utilities|Array|MakeArray (Class|AdvancedSessionsLibrary|MakeLiteralSessionPropertyString "FPSRLGameTag" "FPSRL_v1")) (Game|GetPlayerController 0) 4 0 false true false true true false false false true false true
    (:OnSuccess
      (Variables|SessionRuntimeData|SetbInSession true)
      (Variables|SessionRuntimeData|SetActiveSessionName "GameSession")
      (Game|OpenLevel(byObjectReference) "/Game/MainProject/Contents/Blueprint/Lobby/Lvl_Lobby.Lvl_Lobby" true "listen"))
    (:OnFailure
      (Variables|SessionRuntimeData|SetbInSession false)
      (Development|PrintString "Failed to create Steam session." true true "(R=0.000000,G=0.660000,B=1.000000,A=1.000000)" 5.0))))

(event Custom|FindSessions
  (Variables|SessionSearch|SetbSessionSearchInProgress true)
  (bind _results (|FindSessionsAdvanced (Game|GetPlayerController 0) 50 false "AllServers" 0 false false false)
    (:OnSuccess
      (Variables|SessionSearch|SetbSessionSearchInProgress false)
      (Variables|SessionSearch|SetLastSessionSearchResults _results)
      (Default|CallOnSessionSearchComplete true))
    (:OnFailure
      (Variables|SessionSearch|SetbSessionSearchInProgress false)
      (Default|CallOnSessionSearchComplete false))))

(event Custom|JoinSelectedSession
  (|JoinSession (Game|GetPlayerController 0) (Variables|SessionSearch|GetPendingJoinSessionResult)
    (:OnSuccess
      (Variables|SessionRuntimeData|SetbInSession true)
      (Variables|SessionRuntimeData|SetActiveSessionName "GameSession"))
    (:OnFailure
      (Variables|SessionRuntimeData|SetbInSession false)
      (Development|PrintString "Failed to join the selected session." true true "(R=0.000000,G=0.660000,B=1.000000,A=1.000000)" 5.0))))

(event Custom|InviteFriendToSession
  (Class|AdvancedFriendsLibrary|SendSessionInvitetoFriend (Game|GetPlayerController 0) (Variables|SessionSearch|GetPendingInviteFriendId)
    (:OnSuccess
      (Development|PrintString "Session invite sent." true true "(R=0.000000,G=0.660000,B=1.000000,A=1.000000)" 3.0))
    (:OnFailure
      (Development|PrintString "Failed to send session invite." true true "(R=0.000000,G=0.660000,B=1.000000,A=1.000000)" 3.0))))

(event Custom|LeaveSession
  (|EndSession (Game|GetPlayerController 0)
    (:OnSuccess
      (Variables|SessionRuntimeData|SetbInSession false)
      (Variables|SessionRuntimeData|SetActiveSessionName ""))
    (:OnFailure
      (Development|PrintString "Failed to leave session cleanly." true true "(R=0.000000,G=0.660000,B=1.000000,A=1.000000)" 3.0))))

(event EventOnSessionInviteAccepted
  (params (LocalPlayerNum :type Integer) (PersonInvited :type BP%20Unique%20Net%20Id%20Structure) (SessionToJoin :type Blueprint%20Session%20Result%20Structure%20%28by%20ref%29))
  (|JoinSession (Game|GetPlayerController 0) SessionToJoin
    (:OnSuccess
      (Variables|SessionRuntimeData|SetbInSession true)
      (Variables|SessionRuntimeData|SetActiveSessionName "GameSession"))
    (:OnFailure
      (Variables|SessionRuntimeData|SetbInSession false)
      (Development|PrintString "Failed to join the accepted session invite." true true "(R=0.000000,G=0.660000,B=1.000000,A=1.000000)" 5.0))))