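; Lobby PlayerState Blueprint that holds a player's ready flag, selected weapon index and player index.
; Simple functions toggle readiness, set the weapon selection and return the player index as an identifier.
; The ready flag's OnRep handler is empty, and the event graph has no active logic, only a disconnected copy of the ready toggle.
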(event EventBeginPlay)

(event EventTick
  (params (DeltaSeconds :type Float%20%28single-precision%29)))

(fn ConstructionScript)

(fn OnRepBIsReady)

(fn SetWeaponSelection
  (params (Index :type Byte))
  (Variables|Lobby|SetSelectedWeaponIndex Index))

(fn ToggleReady
  (Variables|Lobby|SetbIsReady (not (Variables|Lobby|GetbIsReady))))

(fn GetPlayerIdentifier
  (return (Variables|Default|GetPlayerIndex)))