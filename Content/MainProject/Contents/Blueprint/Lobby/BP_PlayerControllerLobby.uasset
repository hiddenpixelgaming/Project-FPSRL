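; Lobby player controller that manages input modes, cursor visibility and the crosshair HUD.
; On BeginPlay the local controller adds default, mouse-look and weapon Enhanced Input contexts, and in Lvl_Lobby enters game-only input and creates the crosshair widget.
; Events close the lobby widget or toggle cursor-driven menu mode, ignoring the toggle while Alt is held.
; UpdateCrosshairSpread forwards normalized spread to the crosshair.
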(event Custom|ClientLeaveLobbyUI
  (bind _lobbywidgetinstance (Variables|Default|GetLobbyWidgetInstance))
  (Input|SetInputModeGameOnly self true)
  (Variables|Default|SetbShowMouseCursor false)
  (Utilities|IsValid _lobbywidgetinstance
    (:Is%20Valid
      (Widget|RemovefromParent _lobbywidgetinstance))))

(event Custom|ToggleMenuMode
  (bind _self self)
  (if (not (or (Game|Player|IsInputKeyDown _self "LeftAlt") (Game|Player|IsInputKeyDown _self "RightAlt")))
    (if (Variables|Default|GetbShowMouseCursor)
      (Input|SetInputModeGameOnly _self true)
      (Variables|Default|SetbShowMouseCursor false)
      (else
        (Input|SetInputModeGameandUI _self (Variables|Default|GetLobbyWidgetInstance) "DoNotLock" true true)
        (Variables|Default|SetbShowMouseCursor true)))))

(event EventBeginPlay
  (bind _returnvalue (PlayerController|LocalPlayerSubsystems|GetEnhancedInputLocalPlayerSubsystem))
  (bind _returnvalue_2 (Game|GetCurrentLevelName true))
  (if (Pawn|IsLocalPlayerController)
    (Input|AddMappingContext _returnvalue "/Game/Input/IMC_Default.IMC_Default" 0 "(bIgnoreAllPressedKeysUntilRelease=True,bForceImmediately=False,bNotifyUserSettings=False)")
    (Input|AddMappingContext _returnvalue "/Game/Input/IMC_MouseLook.IMC_MouseLook" 0 "(bIgnoreAllPressedKeysUntilRelease=True,bForceImmediately=False,bNotifyUserSettings=False)")
    (Input|AddMappingContext _returnvalue "/Game/Variant_Shooter/Input/IMC_Weapons.IMC_Weapons" 0 "(bIgnoreAllPressedKeysUntilRelease=True,bForceImmediately=False,bNotifyUserSettings=False)"))
  (if (and (Pawn|IsLocalController) (Utilities|Enum|Equal(Enum) _returnvalue_2 "Lvl_Lobby"))
    (Input|SetInputModeGameOnly self true)
    (Variables|Default|SetbShowMouseCursor false)
    (bind _returnvalue_3 (UserInterface|CreateWidget "/Game/Variant_Shooter/UI/WB_Crosshair.WB_Crosshair_C" self))
    (Variables|Default|SetCrosshairUI _returnvalue_3)
    (UserInterface|Viewport|AddtoViewport _returnvalue_3 0)))

(event EventTick
  (params (DeltaSeconds :type Float%20%28single-precision%29)))

(fn ConstructionScript)

(fn UpdateCrosshairSpread
  (params (NormalizedSpread :type Float%20%28double-precision%29))
  (bind _crosshairui (Variables|Default|GetCrosshairUI))
  (Utilities|IsValid _crosshairui
    (:Is%20Valid
      (Default|SetSpread _crosshairui NormalizedSpread))))