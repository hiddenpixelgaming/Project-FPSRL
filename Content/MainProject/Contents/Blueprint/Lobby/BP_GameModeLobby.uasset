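; BP_GameModeLobby is the lobby game mode, which numbers players as they join.
; On PostLogin it casts the new player's state to BP_PlayerStateLobby and checks its player identifier.
; If that is zero, it writes the NextPlayerIndex counter into PlayerIndex and increments the counter.
; Once the counter passes four it only prints a session-full message, without rejecting the player.
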(event EventBeginPlay)

(event EventTick
  (params (DeltaSeconds :type Float%20%28single-precision%29)))

(event EventPostLogin
  (params (NewPlayer :type Player%20Controller%20Object%20Reference))
  (CallFunction|AssignPlayerIdentifier self NewPlayer))

(fn ConstructionScript)

(fn AssignPlayerIdentifier
  (params (NewPlayer :type Player%20Controller%20Object%20Reference))
  (bind _asbp_player_state_lobby (Utilities|Casting|CastToBP_PlayerStateLobby (Variables|/Script/Engine.Controller|GetPlayerState NewPlayer)))
  (bind _playerindex (Default|GetPlayerIdentifier _asbp_player_state_lobby))
  (if (== _playerindex (Class|KismetSystemLibrary|MakeLiteralInteger))
    (if (> (Variables|Default|GetNextPlayerIndex) (Class|KismetSystemLibrary|MakeLiteralInteger 4))
      (Development|PrintString "Session full: cannot assign a 5th player identifier.")
      (else
        (Variables|/Game/MainProject/Contents/Blueprint/Lobby/BP_PlayerStateLobby.BP_PlayerStateLobby_C|SetPlayerIndex _asbp_player_state_lobby (Variables|Default|GetNextPlayerIndex))
        (Variables|Default|SetNextPlayerIndex (+ (Variables|Default|GetNextPlayerIndex) (Class|KismetSystemLibrary|MakeLiteralInteger 1)))))))