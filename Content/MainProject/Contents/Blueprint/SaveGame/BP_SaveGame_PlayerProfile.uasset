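; BP_SaveGame_PlayerProfile is a player profile save object that tracks collected and equipped relics.
; TryEquipRelic always records the relic as collected, equips it if a slot is free under MaxEquippedRelics, and returns true when slots are full.
; ReplaceRelic swaps an equipped relic for a new one while recording it as collected.
; UnequipRelic removes a relic from the equipped list only, leaving the collection intact.
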(fn TryEquipRelic
  (params (NewRelic :type BP%20Relic%20Base%20Object%20Reference))
  (Utilities|Array|AddUnique (Variables|Default|GetCollectedRelics) NewRelic)
  (if (< (Utilities|Array|Length (Variables|Default|GetEquippedRelics)) (Variables|Default|GetMaxEquippedRelics))
    (Utilities|Array|AddUnique (Variables|Default|GetEquippedRelics) NewRelic)
    (return false)
    (else
      (return true))))

(fn ReplaceRelic
  (params (OldRelic :type BP%20Relic%20Base%20Object%20Reference) (NewRelic :type BP%20Relic%20Base%20Object%20Reference))
  (Utilities|Array|AddUnique (Variables|Default|GetCollectedRelics) NewRelic)
  (Utilities|Array|RemoveItem (Variables|Default|GetEquippedRelics) OldRelic)
  (Utilities|Array|AddUnique (Variables|Default|GetEquippedRelics) NewRelic))

(fn UnequipRelic
  (params (RelicToRemove :type BP%20Relic%20Base%20Object%20Reference))
  (Utilities|Array|RemoveItem (Variables|Default|GetEquippedRelics) RelicToRemove))