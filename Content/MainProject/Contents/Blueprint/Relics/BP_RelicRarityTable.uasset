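; BP_RelicRarityTable holds relic rarity tiers and picks one at random by drop percentage.
; RollRarity adds an optional per-index bonus to each tier's DropPercent, clamps it at zero and sums the weights.
; It rolls within that total and returns the first tier whose running total reaches the roll, falling back to the last tier.
; Because the roll uses the summed weights, percentages need not total 100.
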(fn GetEffectiveWeight
  (params (Tier :type BP%20Relic%20Rarity%20Base%20Object%20Reference) (Bonus :type Float%20%28double-precision%29))
  (return (Math|Float|Max(Float) (+ (Variables|/Game/MainProject/Contents/Blueprint/Relics/BP_RelicRarity_Base.BP_RelicRarity_Base_C|GetDropPercent Tier) Bonus) 0.0)))

(fn RollRarity
  (params (BonusPercents :type Array%20of%20Floats%20%28double-precision%29))
  (bind _raritytiers (Variables|Default|GetRarityTiers))
  (bind _returnvalue (Utilities|Array|Length _raritytiers))
  (LocalVariables|SetTotalWeight 0.0)
  (for _index (range 0 (- _returnvalue (Class|KismetSystemLibrary|MakeLiteralInteger 1)))
    (bind _weight (CallFunction|GetEffectiveWeight (Utilities|Array|Get(acopy) _raritytiers _index) (select (Utilities|Array|IsValidIndex BonusPercents _index) (Utilities|Array|Get(acopy) BonusPercents _index) (Math|Float|MakeLiteralFloat 0.0))))
    (LocalVariables|SetTotalWeight (+ (LocalVariables|GetTotalWeight) _weight)))
  (LocalVariables|SetRoll (Math|Random|RandomFloatinRange 0.0 (LocalVariables|GetTotalWeight)))
  (LocalVariables|SetRunningTotal 0.0)
  (for _index_2 (range 0 (- _returnvalue (Class|KismetSystemLibrary|MakeLiteralInteger 1)))
    (bind _weight_2 (CallFunction|GetEffectiveWeight (Utilities|Array|Get(acopy) _raritytiers _index_2) (select (Utilities|Array|IsValidIndex BonusPercents _index_2) (Utilities|Array|Get(acopy) BonusPercents _index_2) (Math|Float|MakeLiteralFloat 0.0))))
    (LocalVariables|SetRunningTotal (+ (LocalVariables|GetRunningTotal) _weight_2))
    (if (<= (LocalVariables|GetRoll) (LocalVariables|GetRunningTotal))
      (return (Utilities|Array|Get(acopy) _raritytiers _index_2))))
  (return (Utilities|Array|Get(acopy) _raritytiers (- _returnvalue (Class|KismetSystemLibrary|MakeLiteralInteger 1)))))