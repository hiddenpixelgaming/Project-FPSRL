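; Health component that tracks current and max health for its owning actor and handles damage, healing and death.
; Damage and heal functions change health only with authority, clamping it and broadcasting OnDeath with instigator and causer when it reaches zero.
; The CurrentHealth RepNotify broadcasts OnHealthChanged, and helpers report death state and health percent.
; BeginPlay is empty, so no damage binding appears here, and damage and death print debug strings.
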(event EventBeginPlay)

(fn OnRepCurrentHealth
  (Default|CallOnHealthChanged self (Variables|Default|GetCurrentHealth) (Variables|Default|GetMaxHealth)))

(fn Heal
  (params (Amount :type Float%20%28double-precision%29))
  (if (Ability|HasAuthority (Components|GetOwner self))
    (Variables|Default|SetCurrentHealth (Math|Float|Clamp(Float) (+ (Variables|Default|GetCurrentHealth) Amount) 0.0 (Variables|Default|GetMaxHealth)))))

(fn IsDead
  (return (<= (Variables|Default|GetCurrentHealth) 0.0)))

(fn GetHealthPercent
  (return (/ (Variables|Default|GetCurrentHealth) (Variables|Default|GetMaxHealth))))

(fn HandleTakeAnyDamage
  (params (Damage :type Float%20%28double-precision%29) (DamageType :type Damage%20Type%20Object%20Reference) (InstigatedBy :type Controller%20Object%20Reference) (DamageCauser :type Actor%20Object%20Reference))
  (bind _self self)
  (if (Ability|HasAuthority (Components|GetOwner _self))
    (if (> (Variables|Default|GetCurrentHealth) (Math|Float|MakeLiteralFloat 0.0))
      (Variables|Default|SetCurrentHealth (Math|Float|Max(Float) (- (Variables|Default|GetCurrentHealth) Damage) 0.0))
      (Development|PrintString (Utilities|String|Append (Utilities|String|Append (Utilities|GetDisplayName (Components|GetOwner _self)) " took damage. HP now ") (Utilities|String|ToString(Float) (Variables|Default|GetCurrentHealth))))
      (if (<= (Variables|Default|GetCurrentHealth) 0.0)
        (Development|PrintString (Utilities|String|Append (Utilities|GetDisplayName (Components|GetOwner _self)) " DIED (OnDeath broadcasting)") true true "(R=1.0,G=0.0,B=0.0,A=1.0)")
        (Default|CallOnDeath _self InstigatedBy DamageCauser)))))