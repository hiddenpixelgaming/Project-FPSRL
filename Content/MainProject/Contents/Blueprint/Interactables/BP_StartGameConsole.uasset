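; Interactable game console actor that offers BP_ShooterCharacter an "access console" prompt while overlapping; the console action itself is not implemented here.
; Tick polls overlapping characters instead of using overlap events and registers only the first as interactor via SetCurrentInteractable.
; It caches that character to clear the prompt when the overlap ends or the first character changes.
; BeginPlay draws a temporary debug sphere around the actor, independent of detection.
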(event EventBeginPlay
  (Rendering|Debug|DrawDebugSphere (Transformation|GetActorLocation) 2e+02 24 "(R=1.000000,G=1.000000,B=1.000000,A=1.000000)" 3e+02 3.0))

(event Collision|EventActorBeginOverlap
  (params (OtherActor :type Actor%20Object%20Reference)))

(event EventTick
  (params (DeltaSeconds :type Float%20%28single-precision%29))
  (bind _self self)
  (bind _overlappingactors (Collision|GetOverlappingActors _self "/Game/Variant_Shooter/Blueprints/BP_ShooterCharacter.BP_ShooterCharacter_C" :!class /Script/Engine.Actor))
  (bind _output (Utilities|Array|Get(acopy) _overlappingactors))
  (if (> (Utilities|Array|Length _overlappingactors) (Class|KismetSystemLibrary|MakeLiteralInteger))
    (if (!= _output (Variables|Default|GetLastOverlappingCharacter))
      (bind _asbp_shooter_character (Utilities|Casting|CastToBP_ShooterCharacter (Variables|Default|GetLastOverlappingCharacter))
        (:then
          (Default|ClearCurrentInteractable _asbp_shooter_character _self)
          (Variables|Default|SetLastOverlappingCharacter _output)
          (bind _asbp_shooter_character_2 (Utilities|Casting|CastToBP_ShooterCharacter _output))
          (Default|SetCurrentInteractable _asbp_shooter_character_2 _self "Press E to Access Game Console"))
        (:CastFailed
          (Variables|Default|SetLastOverlappingCharacter _output)
          (bind _asbp_shooter_character_3 (Utilities|Casting|CastToBP_ShooterCharacter _output))
          (Default|SetCurrentInteractable _asbp_shooter_character_3 _self "Press E to Access Game Console"))))
    (else
      (bind _asbp_shooter_character_4 (Utilities|Casting|CastToBP_ShooterCharacter (Variables|Default|GetLastOverlappingCharacter)))
      (Default|ClearCurrentInteractable _asbp_shooter_character_4 _self)
      (Variables|Default|SetLastOverlappingCharacter 0))))

(fn ConstructionScript)